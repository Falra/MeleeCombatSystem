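; BP_MasterPose is an item actor in the combat system for skeletal meshes that animate along with their owning character.
; Its AttachActor function snaps a valid ItemSkeletalMesh to a given socket on the owner Character's mesh.
; It then sets that mesh as leader pose component, so the item copies the character's pose.
; The event graph is unused.
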(fn `AttachActor`
  (params (SocketName :type Name))
  (bind _mesh (`Character.Mesh` (cast `Character` (`self.GetOwner`) :!pure true)))
  (bind _itemskeletalmesh (`self.ItemSkeletalMesh`)
    (:`then`
      (`SceneComponent.K2_AttachToComponent` _itemskeletalmesh _mesh SocketName "SnapToTarget" "SnapToTarget" "SnapToTarget" true)
      (`SkinnedMeshComponent.SetLeaderPoseComponent` (`self.ItemSkeletalMesh`) _mesh false false)
      (return))
    (:`else`
      (return))))

(fn `UserConstructionScript`
  (`parent.UserConstructionScript`))