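; Base actor for equippable items in the combat system, tracking whether the item is equipped.
; On equip it sets the Equipped flag and snaps itself to a named socket on the owning Character's mesh.
; Unequip only clears the flag, without detaching.
; GetItemMesh returns the static mesh component when it has a valid mesh, otherwise the skeletal one.
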(fn `AttachActor`
  (params (SocketName :type Name))
  (`self.K2_AttachToComponent` (`Character.Mesh` (cast `Character` (`self.GetOwner`) :!pure true)) SocketName "SnapToTarget" "SnapToTarget" "SnapToTarget"))

(fn `GetItemMesh`
  (returns (ItemMesh :type "PrimitiveComponent Object Reference"))
  (bind _itemstaticmesh (`self.ItemStaticMesh`))
  (`StaticMeshComponent.StaticMesh` _itemstaticmesh
    (:`then`
      (return _itemstaticmesh))
    (:`else`
      (return (`self.ItemSkeletalMesh`)))))

(fn `OnEquipped`
  (set `self.bEquipped` true)
  (`self.AttachActor` (`self.Attach Socket Name`)))

(fn `OnUnequipped`
  (if (`self.bEquipped`)
    (set `self.bEquipped` false)))

(fn `UserConstructionScript`)