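; Base actor for dual-wielded weapons in the combat system, extending its parent weapon with a second mesh and collision component for the off hand.
; Activating or deactivating collision switches on the collision part, toggling either the main or second weapon's collision component independently.
; On equip, it runs the parent logic, then assigns the second mesh to the second collision component.
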(fn `ActivateCollision`
  (params (CollisionPart :type "/Game/CombatSystem/Blueprints/Enums/E_CollisionPart Enum" :default "NewEnumerator0"))
  (switch `/Game/CombatSystem/Blueprints/Enums/E_CollisionPart` CollisionPart
    (:`NewEnumerator0`
      (`/Game/CombatSystem/Blueprints/Components/BP_CollisionComponent.EnableCollision` (`self.MainWeaponCollisionComponent`)))
    (:`NewEnumerator1`
      (`/Game/CombatSystem/Blueprints/Components/BP_CollisionComponent.EnableCollision` (`self.SecondWeaponCollisionComponent`)))))

(fn `DeactivateCollision`
  (params (CollisionPart :type "/Game/CombatSystem/Blueprints/Enums/E_CollisionPart Enum" :default "NewEnumerator0"))
  (switch `/Game/CombatSystem/Blueprints/Enums/E_CollisionPart` CollisionPart
    (:`NewEnumerator0`
      (`/Game/CombatSystem/Blueprints/Components/BP_CollisionComponent.DisableCollision` (`self.MainWeaponCollisionComponent`)))
    (:`NewEnumerator1`
      (`/Game/CombatSystem/Blueprints/Components/BP_CollisionComponent.DisableCollision` (`self.SecondWeaponCollisionComponent`)))))

(fn `OnEquipped`
  (`parent.OnEquipped`)
  (`/Game/CombatSystem/Blueprints/Components/BP_CollisionComponent.SetCollisionMeshComponent` (`self.SecondWeaponCollisionComponent`) (`self.SecondMesh`)))

(fn `UserConstructionScript`
  (`parent.UserConstructionScript`))