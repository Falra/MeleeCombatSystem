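; AN_ToggleCombat is an animation notify that sheathes or draws the owner's main weapon and toggles combat mode.
; It finds the BP_CombatComponent on the mesh owner and, if a main weapon is valid, attaches it to either its hand socket or its attach socket based on the AttachToHand flag.
; The same flag then sets whether combat is enabled on the component.
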(fn `Received_Notify`
  (params (MeshComp :type "SkeletalMeshComponent Object Reference") (Animation :type "AnimSequenceBase Object Reference") (EventReference :type "AnimNotifyEventReference Structure (by ref)"))
  (returns (ReturnValue :type Boolean))
  (locals (CombatComponent :type "/Game/CombatSystem/Blueprints/Components/BP_CombatComponent Object Reference"))
  (bind _output_get (set `local.CombatComponent` (`Actor.GetComponentByClass` (`ActorComponent.GetOwner` MeshComp) "/Game/CombatSystem/Blueprints/Components/BP_CombatComponent.BP_CombatComponent_C")))
  (bind _mainweapon (`/Game/CombatSystem/Blueprints/Components/BP_CombatComponent.GetMainWeapon` _output_get))
  (`/Engine/EditorBlueprintResources/StandardMacros.IsValid` _mainweapon
    (:`Is Valid`
      (`/Game/CombatSystem/Blueprints/Actors/BP_BaseEquippable.AttachActor` _mainweapon (select `bool` (`self.AttachToHand`) :`false` (`/Game/CombatSystem/Blueprints/Actors/BP_BaseEquippable.Attach Socket Name` _mainweapon) :`true` (`/Game/CombatSystem/Blueprints/Actors/BP_BaseWeapon.HandSocketName` _mainweapon)))
      (`/Game/CombatSystem/Blueprints/Components/BP_CombatComponent.SetCombatEnabled` (`local.CombatComponent`) (`self.AttachToHand`))
      (return true))
    (:`Is Not Valid`
      (return false))))