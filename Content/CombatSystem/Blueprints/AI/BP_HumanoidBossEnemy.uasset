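; Humanoid boss enemy for the combat system, extending its parent AI character with a weapon mesh and an on-screen boss health bar.
; On begin play it registers the weapon mesh for collision and creates the health widget from its stats component.
; Targeting events toggle the bar's visibility, and combat toggles snap the weapon between hand and attach sockets.
; Death enables physics on the weapon and removes the bar.
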(event `self.ReceiveBeginPlay`
  (`parent.ReceiveBeginPlay`)
  (`/Game/CombatSystem/Blueprints/Components/BP_CollisionComponent.SetCollisionMeshComponent` (`self.MainWeaponCollisionComponent`) (`self.WeaponMesh`))
  (bind _returnvalue (`|CreateWidget` "/Game/CombatSystem/UI/WBP_BossHealth.WBP_BossHealth_C" (`GameplayStatics.GetPlayerController` 0)))
  (set `self.BossHealthUI` _returnvalue)
  (`/Game/CombatSystem/UI/WBP_BossHealth.Initialize` _returnvalue (`self.StatsComponent`))
  (`UserWidget.AddToViewport` (`self.BossHealthUI`) 0))

(event `self.OnTargeted`
  (params (bTargeted :type Boolean))
  (`parent.OnTargeted` bTargeted)
  (`self.SetBossHealthVisibility` bTargeted))

(event `SetBossHealthVisibility`
  (params (NewVisibility :type Boolean))
  (bind _bosshealthui (`self.BossHealthUI`)
    (:`then`
      (`Widget.SetVisibility` _bosshealthui (select `bool` NewVisibility :`false` "Hidden" :`true` "Visible" :!type "ESlateVisibility Enum")))
    (:`else`)))

(event `SimulateWeaponPhysics`
  (bind _weaponmesh (`self.WeaponMesh`))
  (`PrimitiveComponent.SetCollisionProfileName` _weaponmesh "PhysicsActor" true)
  (`PrimitiveComponent.SetSimulatePhysics` _weaponmesh true))

(event `self.PerformDeath`
  (`parent.PerformDeath`)
  (`self.SimulateWeaponPhysics`)
  (bind _bosshealthui (`self.BossHealthUI`)
    (:`then`
      (`Widget.RemoveFromParent` _bosshealthui))
    (:`else`)))

(event `self.ToggleCombat`
  (params (bEnableCombat :type Boolean))
  (`parent.ToggleCombat` bEnableCombat)
  (`SceneComponent.K2_AttachToComponent` (`self.WeaponMesh`) (`self.Mesh`) (select `bool` bEnableCombat :`false` (`self.Attach Socket Name`) :`true` (`self.HandSocketName`)) "SnapToTarget" "SnapToTarget" "SnapToTarget" true))

(event `self.OnTargetSet`
  (params (NewTarget :type "Actor Object Reference"))
  (`parent.OnTargetSet` NewTarget)
  (`self.SetBossHealthVisibility` (`KismetSystemLibrary.IsValid` NewTarget)))

(fn `UserConstructionScript`
  (`parent.UserConstructionScript`))