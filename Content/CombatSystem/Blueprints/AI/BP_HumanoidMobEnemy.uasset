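; BP_HumanoidMobEnemy is a humanoid enemy that extends its parent's combat behavior with a visible weapon and a health bar.
; On BeginPlay it binds the weapon mesh to the weapon collision component and builds a health bar widget from its own stats component, shown or hidden with targeting.
; Toggling combat snaps the weapon between hand and attach sockets.
; On death the weapon switches to physics simulation.
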(event `self.ReceiveBeginPlay`
  (`parent.ReceiveBeginPlay`)
  (`/Game/CombatSystem/Blueprints/Components/BP_CollisionComponent.SetCollisionMeshComponent` (`self.MainWeaponCollisionComponent`) (`self.WeaponMesh`))
  (bind _returnvalue (`|CreateWidget` "/Game/CombatSystem/UI/WBP_EnemyHeathBar.WBP_EnemyHeathBar_C" (`GameplayStatics.GetPlayerController` 0) (`self.StatsComponent`) false))
  (`WidgetComponent.SetWidget` (`self.HealthWidget`) _returnvalue))

(event `/Game/CombatSystem/Blueprints/Interfaces/BPI_Targeting.OnTargeted`
  (params (bTargeted :type Boolean))
  (`parent.OnTargeted` bTargeted)
  (`SceneComponent.SetVisibility` (`self.HealthWidget`) bTargeted false))

(event `SimulateWeaponPhysics`
  (bind _weaponmesh (`self.WeaponMesh`))
  (`PrimitiveComponent.SetCollisionProfileName` _weaponmesh "PhysicsActor" true)
  (`PrimitiveComponent.SetSimulatePhysics` _weaponmesh true))

(event `self.PerformDeath`
  (`parent.PerformDeath`)
  (`self.SimulateWeaponPhysics`))

(event `/Game/CombatSystem/Blueprints/Interfaces/BPI_Combat.ToggleCombat`
  (params (bEnableCombat :type Boolean))
  (`parent.ToggleCombat` bEnableCombat)
  (`SceneComponent.K2_AttachToComponent` (`self.WeaponMesh`) (`self.Mesh`) (select `bool` bEnableCombat :`false` (`self.Attach Socket Name`) :`true` (`self.HandSocketName`)) "SnapToTarget" "SnapToTarget" "SnapToTarget" true))

(fn `UserConstructionScript`
  (`parent.UserConstructionScript`))