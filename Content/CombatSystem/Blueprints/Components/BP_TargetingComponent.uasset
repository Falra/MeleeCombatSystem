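; Actor component that provides lock-on targeting for a Character owner in the combat system.
; Enable, disable and toggle events set or clear the targeting flag and the stored target actor.
; Target search sphere-traces from the owner's location along the follow camera's forward vector, filtered by object type, and takes the single hit actor.
; It only holds lock-on state; camera or character rotation is not driven here.
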(event `self.ReceiveBeginPlay`
  (`parent.ReceiveBeginPlay`)
  (bind _ascharacter (cast `Character` (`self.GetOwner`)))
  (bind _output_get (set `self.OwnerCharacter` _ascharacter))
  (set `self.OwnerController` (`Pawn.GetController` _output_get))
  (set `self.FollowCamera` (`Actor.GetComponentByClass` (`self.OwnerCharacter`) "/Script/Engine.CameraComponent")))

(event `EnableLockOn`
  (bind (_returnvalue _target) (`self.FindTarget`))
  (if _returnvalue
    (`self.SetTargetActor` _target)
    (`self.SetTargetting` true)))

(event `DisableLockOn`
  (`self.SetTargetting` false)
  (`self.SetTargetActor` null))

(event `ToggleLockOn`
  (if (not (`self.IsTargetting`))
    (`self.EnableLockOn`)
    (else
      (`self.DisableLockOn`))))

(fn `FindTarget`
  (returns (ReturnValue :type Boolean) (Target :type "Actor Object Reference"))
  (bind _returnvalue (`Actor.K2_GetActorLocation` (`self.GetOwner`)))
  (bind (_outhit _returnvalue_2) (`KismetSystemLibrary.SphereTraceSingleForObjects` _returnvalue (+ _returnvalue (* (`SceneComponent.GetForwardVector` (`self.FollowCamera`)) (`self.TargetingDistance`))) (`self.TargetingRadius`) (`self.Target Object Types`) false (`|MakeArray` (`self.GetOwner`))))
  (bind (_bblockinghit _binitialoverlap _time _distance _location _impactpoint _normal _impactnormal _physmat _hitactor) (`GameplayStatics.BreakHitResult` _outhit))
  (if (and _returnvalue_2 (`KismetSystemLibrary.IsValid` _hitactor))
    (return true _hitactor)
    (else
      (return false null))))

(fn `GetTargetActor`
  (returns (TargetActor :type "Actor Object Reference"))
  (return (`self.TargetActor`)))

(fn `IsTargetting`
  (returns (bTargeting :type Boolean))
  (return (`self.bTargeting`)))

(fn `SetTargetActor`
  (params (NewTargetActor :type "Actor Object Reference"))
  (set `self.TargetActor` NewTargetActor))

(fn `SetTargetting`
  (params (bEnableTargeting :type Boolean))
  (set `self.bTargeting` bEnableTargeting))