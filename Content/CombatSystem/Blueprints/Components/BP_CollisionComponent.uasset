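; BP_CollisionComponent is a combat component that detects hits along a mesh with socket-to-socket traces.
; While collision is enabled, each Tick runs a multi-sphere object trace between the mesh's start and end sockets, skipping ignored actors.
; Newly hit actors are recorded and fire OnHit, so each triggers only once until the hit list is cleared, which also happens whenever collision is enabled.
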(event `EnableCollision`
  (`self.ClearHitActors`)
  (set `self.bCollisionEnabled` true))

(event `DisableCollision`
  (set `self.bCollisionEnabled` false))

(event `CollisionTrace`
  (bind _collisionmeshcomponent (`self.CollisionMeshComponent`))
  (bind _outhits (`KismetSystemLibrary.SphereTraceMultiForObjects` (`SceneComponent.GetSocketLocation` _collisionmeshcomponent (`self.Start Socket Name`)) (`SceneComponent.GetSocketLocation` _collisionmeshcomponent (`self.End Socket Name`)) (`self.TraceRadius`) (`self.Trace Object Types`) false (`self.Actors to Ignore`) (`self.Draw Debug Type`)))
  (for _array_element _outhits
    (bind _output_get (set `self.LastHit` _array_element))
    (bind (_bblockinghit _binitialoverlap _time _distance _location _impactpoint _normal _impactnormal _physmat _hitactor) (`GameplayStatics.BreakHitResult` _output_get))
    (if (not (`KismetArrayLibrary.Array_Contains` (`self.HitActors`) _hitactor))
      (bind _output_get_2 (set `self.Hit Actor` _hitactor))
      (`KismetArrayLibrary.Array_Add` (`self.HitActors`) _output_get_2)
      (`self.OnHit` (`self.LastHit`)))))

(event `ClearHitActors`
  (`KismetArrayLibrary.Array_Clear` (`self.HitActors`)))

(event `self.ReceiveTick`
  (params (DeltaSeconds :type "Float (single-precision)"))
  (if (`self.bCollisionEnabled`)
    (`self.CollisionTrace`)))

(event `SetCollisionMeshComponent`
  (params (MeshComponent :type "PrimitiveComponent Object Reference"))
  (set `self.CollisionMeshComponent` MeshComponent))

(fn `AddActorToIgnore`
  (params (InActor :type "Actor Object Reference (by ref)"))
  (`KismetArrayLibrary.Array_AddUnique` (`self.Actors to Ignore`) InActor))

(fn `GetActorsToIgnore`
  (returns (`Actors to Ignore` :type "Array of Actor Object Reference"))
  (return (`self.Actors to Ignore`)))

(fn `GetHitActors`
  (returns (HitActors :type "Array of Actor Object Reference"))
  (return (`self.HitActors`)))

(fn `GetLastHit`
  (returns (LastHit :type "HitResult Structure"))
  (return (`self.LastHit`)))

(fn `GetMeshComponent`
  (returns (MeshComponent :type "PrimitiveComponent Object Reference"))
  (return (`self.CollisionMeshComponent`)))

(fn `IsCollisionEnabled`
  (returns (bCollisionEnabled :type Boolean))
  (return (`self.bCollisionEnabled`)))

(fn `RemoveActorToIgnore`
  (params (InActor :type "Actor Object Reference (by ref)"))
  (`KismetArrayLibrary.Array_RemoveItem` (`self.Actors to Ignore`) InActor))