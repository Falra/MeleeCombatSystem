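; BP_StatsComponent is a combat component that tracks a set of stats, each with a base, max and current value.
; InitializeStats fills the CurrentStats map from the base values in the BaseStats struct map, and getters and setters expose each value by stat key.
; ModifyCurrentStatValue applies deltas clamped between zero and max.
; TakeDamage subtracts damage from one fixed stat through it and returns whether that stat has reached zero.
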(fn `GetBaseStatValue`
  (params (Stat :type "/Game/CombatSystem/Blueprints/Enums/E_Stats Enum" :default "NewEnumerator0"))
  (returns (Value :type "Float (double-precision)"))
  (return (break `/Game/CombatSystem/Blueprints/Structs/F_BaseStat` (`BlueprintMapLibrary.Map_Find` (`self.BaseStats`) Stat))))

(fn `GetCurrentStatValue`
  (params (Stat :type "/Game/CombatSystem/Blueprints/Enums/E_Stats Enum" :default "NewEnumerator0"))
  (returns (Value :type "Float (double-precision)"))
  (return (`BlueprintMapLibrary.Map_Find` (`self.CurrentStats`) Stat)))

(fn `GetMaxStatValue`
  (params (Stat :type "/Game/CombatSystem/Blueprints/Enums/E_Stats Enum" :default "NewEnumerator0"))
  (returns (Value :type "Float (double-precision)"))
  (return (`.MaxValue_4_C67AACC54D9A0CA8E18E5B959CD22FD8` (break `/Game/CombatSystem/Blueprints/Structs/F_BaseStat` (`BlueprintMapLibrary.Map_Find` (`self.BaseStats`) Stat)))))

(fn `InitializeStats`
  (bind _keys (`BlueprintMapLibrary.Map_Keys` (`self.BaseStats`)))
  (for _array_element _keys
    (`self.SetCurrentStatValue` _array_element (break `/Game/CombatSystem/Blueprints/Structs/F_BaseStat` (`BlueprintMapLibrary.Map_Find` (`self.BaseStats`) _array_element)))))

(fn `ModifyCurrentStatValue`
  (params (Stat :type "/Game/CombatSystem/Blueprints/Enums/E_Stats Enum" :default "NewEnumerator0") (ValueDelta :type "Float (double-precision)"))
  (locals (L_Value :type "Float (double-precision)"))
  (if (!= ValueDelta 0.0)
    (bind _output_get (set `local.L_Value` (`KismetMathLibrary.FClamp` (+ (`self.GetCurrentStatValue` (`local.Stat`)) (`local.ValueDelta`)) 0.0 (`self.GetMaxStatValue` (`local.Stat`)))))
    (`self.SetCurrentStatValue` (`local.Stat`) _output_get)))

(fn `SetBaseStatValue`
  (params (Stat :type "/Game/CombatSystem/Blueprints/Enums/E_Stats Enum" :default "NewEnumerator0") (Value :type "Float (double-precision)"))
  (bind _structout (setmembers `/Game/CombatSystem/Blueprints/Structs/F_BaseStat` :`StructRef` (`BlueprintMapLibrary.Map_Find` (`self.BaseStats`) (`local.Stat`)) :`BaseValue` Value))
  (`BlueprintMapLibrary.Map_Add` (`self.BaseStats`) (`local.Stat`) _structout))

(fn `SetCurrentStatValue`
  (params (Stat :type "/Game/CombatSystem/Blueprints/Enums/E_Stats Enum" :default "NewEnumerator0") (Value :type "Float (double-precision)"))
  (`BlueprintMapLibrary.Map_Add` (`self.CurrentStats`) Stat Value))

(fn `SetMaxStatValue`
  (params (Stat :type "/Game/CombatSystem/Blueprints/Enums/E_Stats Enum" :default "NewEnumerator0") (Value :type "Float (double-precision)"))
  (bind _structout (setmembers `/Game/CombatSystem/Blueprints/Structs/F_BaseStat` :`StructRef` (`BlueprintMapLibrary.Map_Find` (`self.BaseStats`) (`local.Stat`)) :`MaxValue` Value))
  (`BlueprintMapLibrary.Map_Add` (`self.BaseStats`) (`local.Stat`) _structout))

(fn `TakeDamage`
  (params (Damage :type "Float (double-precision)"))
  (returns (bDead :type Boolean))
  (`self.ModifyCurrentStatValue` "NewEnumerator1" (* Damage -1.0))
  (return (<= (`self.GetCurrentStatValue` "NewEnumerator1") 0.0)))